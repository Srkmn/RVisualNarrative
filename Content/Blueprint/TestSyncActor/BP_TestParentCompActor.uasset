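; BP_TestParentCompActor is a test actor that shows a boolean dialogue value through the color of an arrow.
; On BeginPlay it adds a component of ParentCompClass at runtime and stores it as ParentCompObj.
; Every Tick it gets the dialogue manager from that component, reads the value named "1" as a bool, and sets the arrow green when true, red when false.
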(event `self.ReceiveBeginPlay`
  (bind _returnvalue (`|AddComponentByClass` (`self.ParentCompClass`)))
  (set `self.ParentCompObj` _returnvalue))

(event `self.ReceiveTick`
  (params (DeltaSeconds :type "Float (single-precision)"))
  (bind _returnvalue (`RVNComponent.GetDialogueManager` (`self.ParentCompObj`)))
  (`ArrowComponent.SetArrowColor` (`self.Arrow`) (`KismetMathLibrary.SelectColor` (make `LinearColor` 0.0 255.0 0.0 255.0) (make `LinearColor` 255.0 0.0 0.0 255.0) (`RVNDialogueManager.GetValueAsBool` _returnvalue "1"))))

(fn `UserConstructionScript`)