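; BP_OtherNPC is an NPC actor whose arrow component visualizes a boolean state from the dialogue system.
; On BeginPlay it adds a component at runtime and stores it to reach its dialogue manager.
; Every Tick it reads a named bool from that manager and colors the arrow green when true, red otherwise.
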(event `self.ReceiveBeginPlay`
  (bind _returnvalue (`|AddComponentByClass` (`self.1`)))
  (bind _output_get (set `self.2` _returnvalue))
  (`RVNComponent.GetDialogueManager` _output_get))

(event `self.ReceiveTick`
  (params (DeltaSeconds :type "Float (single-precision)"))
  (bind _arrow (`self.Arrow`))
  (bind _returnvalue (`RVNComponent.GetDialogueManager` (`self.2`)))
  (if (`RVNDialogueManager.GetValueAsBool` _returnvalue "1")
    (`ArrowComponent.SetArrowColor` _arrow (struct :`R` 0.155539 :`G` 1.0 :`A` 1.0))
    (else
      (`ArrowComponent.SetArrowColor` _arrow (struct :`R` 1.0 :`B` 0.003645 :`A` 1.0)))))

(fn `UserConstructionScript`)